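; Camera actor Blueprint that auto-scrolls its view along the negative world Y axis at a gradually increasing speed.
; While ScrollActive is set, Tick moves the CameraComponent by a delta-time-scaled step times Multiplier.
; A timer raises Multiplier every few seconds, so scrolling speeds up steadily.
; The ToggleScrollActive event switches scrolling on and off.
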(event Custom|ToggleScrollActive
  (if (Variables|Default|GetScrollActive)
    (Variables|Default|SetScrollActive false)
    (else
      (Variables|Default|SetScrollActive true))))

(event EventBeginPlay)

(event EventActorBeginOverlap
  (params (OtherActor :type Actor%20Object%20Reference)))

(event EventTick
  (params (DeltaSeconds :type Float%20%28single-precision%29))
  (bind _cameracomponent (Variables|CameraActor|GetCameraComponent))
  (bind _returnvalue (Transformation|GetWorldLocation _cameracomponent))
  (if (Variables|Default|GetScrollActive)
    (Transformation|SetWorldLocation _cameracomponent (Math|Vector|MakeVector (.x _returnvalue) (+ (* (* DeltaSeconds (Variables|Default|GetMultiplier)) -1e+02) (.y _returnvalue)) (.z _returnvalue)) false false)
    (bind _output_get (Variables|Default|SetTimer (+ (stale _output_get) DeltaSeconds)))
    (if (> _output_get 3.0)
      (Variables|Default|SetMultiplier (+ (Variables|Default|GetMultiplier) 0.3))
      (Variables|Default|SetTimer 0.0))))

(fn ConstructionScript)