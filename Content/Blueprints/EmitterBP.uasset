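; EmitterBP is an actor holding nine particle system components that the player switches on and off as a group.
; Pressing the LeftCtrl input action flips the IsActive flag and applies it to all nine systems at once, without resetting them.
; BeginPlay, overlap, Tick and the construction script do nothing.
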(event `self.ReceiveBeginPlay`)

(event `self.ReceiveActorBeginOverlap`
  (params (OtherActor :type "Actor Object Reference")))

(event `self.ReceiveTick`
  (params (DeltaSeconds :type "Float (single-precision)")))

(event `InputAction|LeftCtrl`
  (params (Key :type "Key Structure" :default "AnyKey"))
  (:`Pressed`
    (if (`self.IsActive`)
      (set `self.IsActive` false)
      (else
        (set `self.IsActive` true)))
    (`ActorComponent.SetActive` (`self.ParticleSystem`) (`self.IsActive`) false)
    (`ActorComponent.SetActive` (`self.ParticleSystem1`) (`self.IsActive`) false)
    (`ActorComponent.SetActive` (`self.ParticleSystem 2`) (`self.IsActive`) false)
    (`ActorComponent.SetActive` (`self.ParticleSystem3`) (`self.IsActive`) false)
    (`ActorComponent.SetActive` (`self.ParticleSystem4`) (`self.IsActive`) false)
    (`ActorComponent.SetActive` (`self.ParticleSystem6`) (`self.IsActive`) false)
    (`ActorComponent.SetActive` (`self.ParticleSystem7`) (`self.IsActive`) false)
    (`ActorComponent.SetActive` (`self.ParticleSystem8`) (`self.IsActive`) false)
    (`ActorComponent.SetActive` (`self.ParticleSystem5`) (`self.IsActive`) false)))

(fn `UserConstructionScript`)