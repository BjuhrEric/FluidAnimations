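; GameplayPawn_BP is the gameplay pawn that opens the pause menu and runs cleanup when play ends.
; Pressing Space creates the PauseMenu widget if the stored reference is invalid, switches the player to UI-only input, adds the menu to the viewport and pauses the game.
; EndPlay calls CleanUpLF, while BeginPlay, Tick, overlap and the construction script are empty.
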(event `self.ReceiveBeginPlay`)

(event `self.ReceiveActorBeginOverlap`
  (params (OtherActor :type "Actor Object Reference")))

(event `self.ReceiveTick`
  (params (DeltaSeconds :type "Float (single-precision)")))

(event `Key|SpaceBar`
  (params (Key :type "Key Structure" :default "AnyKey"))
  (bind _pausemenuref (`self.PauseMenuRef`))
  (:`Pressed`
    (`/Engine/EditorBlueprintResources/StandardMacros.IsValid` (`self.PauseMenuRef`)
      (:`Is Valid`
        _)
      (:`Is Not Valid`
        (bind _returnvalue (`|CreateWidget` "/Game/Menu/PauseMenu.PauseMenu_C"))
        (set `self.PauseMenuRef` _returnvalue)))
    (`WidgetBlueprintLibrary.SetInputMode_UIOnlyEx` (`GameplayStatics.GetPlayerController` 0) _pausemenuref)
    (`UserWidget.AddToViewport` _pausemenuref 0)
    (`GameplayStatics.SetGamePaused` true)))

(event `self.ReceiveEndPlay`
  (params (EndPlayReason :type "EEndPlayReason Enum" :default "Destroyed"))
  (`self.CleanUpLF`))

(fn `UserConstructionScript`)